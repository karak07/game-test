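; BP_RemoteBomb is a bomb that explodes after its detonation time or when it takes any damage.
; BeginPlay starts a one-shot timer and binds the damage event, with both routes calling Explode.
; The Explode override runs the parent's explosion, then clears and invalidates the timer handle, which cancels the pending timed blast when something else set the bomb off.
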(event `self.ReceiveBeginPlay`
  ;[1 1 1] Timed explosion set up
  (`parent.ReceiveBeginPlay`)
  (bind _returnvalue (`KismetSystemLibrary.K2_SetTimerDelegate` (delegate `TimerExplode`) (`self.TimeToDetonation`)))
  (set `self.BombTimer` _returnvalue)
  ;[1 1 1] Explosion on damage taken (from other bomb)
  (add `self.OnTakeAnyDamage` (delegate `OnDmgRecieved`)))

(event `OnDmgRecieved` :!signature `self.OnTakeAnyDamage`
  (params (DamagedActor :type "Actor Object Reference") (Damage :type "Float (double-precision)") (DamageType :type "DamageType Object Reference") (InstigatedBy :type "Controller Object Reference") (DamageCauser :type "Actor Object Reference"))
  ;[1 1 1] Explosion on damage taken (from other bomb)
  (`self.Explode`))

(event `TimerExplode`
  ;[1 1 1] Timed explosion set up
  (`self.Explode`))

(event `self.Explode`
  ;[1 1 1] Clear timed explosion when exploding (important if due to different reason)
  (`parent.Explode`)
  (`KismetSystemLibrary.K2_ClearAndInvalidateTimerHandle` (`self.BombTimer`)))

(fn `UserConstructionScript`)