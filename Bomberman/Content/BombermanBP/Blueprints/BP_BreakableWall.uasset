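; Destructible wall for a Bomberman-style game that may leave a power-up behind when destroyed.
; On BeginPlay it binds to its own any-damage event, so any damage triggers a drop roll and then destroys the actor.
; MaybeDropPowerUp has a fixed chance to spawn one randomly chosen bomb-count, bomb-range, speed or remote-detonator pickup at the wall's XY position and a fixed height.
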(event `self.ReceiveBeginPlay`
  (add `self.OnTakeAnyDamage` (delegate `OnDmgRecieved`)))

(event `OnDmgRecieved` :!signature `self.OnTakeAnyDamage`
  (params (DamagedActor :type "Actor Object Reference") (Damage :type "Float (double-precision)") (DamageType :type "DamageType Object Reference") (InstigatedBy :type "Controller Object Reference") (DamageCauser :type "Actor Object Reference"))
  (`self.MaybeDropPowerUp`)
  (`self.K2_DestroyActor`))

(fn `MaybeDropPowerUp`
  (bind _returnvalue (`KismetMathLibrary.Conv_VectorToTransform` (`KismetMathLibrary.MakeVector` (.x (.location (`self.GetTransform`))) (.y (.location (`self.GetTransform`))) 90.0)))
  (if (<= (`KismetMathLibrary.RandomFloatInRange` 0.0 1.0) 0.3)
    (switch `int` (`KismetMathLibrary.RandomIntegerInRange` 0 3)
      (:`0`
        (`|SpawnActorFromClass` "/Game/BombermanBP/Blueprints/BP_PowerUpBombsCount.BP_PowerUpBombsCount_C" _returnvalue "Undefined" "OverrideRootScale" null null))
      (:`1`
        (`|SpawnActorFromClass` "/Game/BombermanBP/Blueprints/BP_PowerUpBombsRange.BP_PowerUpBombsRange_C" _returnvalue "Undefined" "OverrideRootScale" null null))
      (:`2`
        (`|SpawnActorFromClass` "/Game/BombermanBP/Blueprints/BP_PowerUpSpeed.BP_PowerUpSpeed_C" _returnvalue "Undefined" "OverrideRootScale" null null))
      (:`3`
        (`|SpawnActorFromClass` "/Game/BombermanBP/Blueprints/BP_PowerUpRemoteDetonator.BP_PowerUpRemoteDetonator_C" _returnvalue "Undefined" "OverrideRootScale" null null)))))

(fn `UserConstructionScript`)