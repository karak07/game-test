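; Player character Blueprint for a Bomberman game, handling death and power-up pickups.
; Any damage takes the player out by hiding the capsule and its children, disabling collision and stopping movement, without destroying the actor.
; A cast chain on overlap applies bomb count, bomb range, walk speed or remote detonator power-ups, then destroys the pickup.
; The remote detonator is temporary, switched off by a one-shot timer.
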(event `self.ReceiveBeginPlay`
  (add `self.OnTakeAnyDamage` (delegate `OnDmgRecieved`)))

(event `OnDmgRecieved` :!signature `self.OnTakeAnyDamage`
  (params (DamagedActor :type "Actor Object Reference") (Damage :type "Float (double-precision)") (DamageType :type "DamageType Object Reference") (InstigatedBy :type "Controller Object Reference") (DamageCauser :type "Actor Object Reference"))
  (`SceneComponent.SetVisibility` (`self.CapsuleComponent`) false true)
  (`self.SetActorEnableCollision` false)
  (`CharacterMovementComponent.DisableMovement` (`self.CharacterMovement`)))

(event `self.ReceiveActorBeginOverlap`
  (params (OtherActor :type "Actor Object Reference"))
  (bind _charactermovement (`self.CharacterMovement`))
  (bind _asbp_power_up_bombs_count (cast `/Game/BombermanBP/Blueprints/BP_PowerUpBombsCount` OtherActor)
    (:`then`
      (`self.IncrementBombCount`)
      (`self.K2_DestroyActor` _asbp_power_up_bombs_count))
    (:`CastFailed`
      (bind _asbp_power_up_bombs_range (cast `/Game/BombermanBP/Blueprints/BP_PowerUpBombsRange` OtherActor)
        (:`then`
          (`self.IncrementBombRange`)
          (`self.K2_DestroyActor` _asbp_power_up_bombs_range))
        (:`CastFailed`
          (bind _asbp_power_up_speed (cast `/Game/BombermanBP/Blueprints/BP_PowerUpSpeed` OtherActor)
            (:`then`
              (set `CharacterMovementComponent.MaxWalkSpeed` (+ (`CharacterMovementComponent.MaxWalkSpeed` _charactermovement) 100.0) _charactermovement)
              (`self.K2_DestroyActor` _asbp_power_up_speed))
            (:`CastFailed`
              (bind _asbp_power_up_remote_detonator (cast `/Game/BombermanBP/Blueprints/BP_PowerUpRemoteDetonator` OtherActor))
              (`self.SetRemoteDetonatorActive` true)
              (`KismetSystemLibrary.K2_SetTimerDelegate` (delegate `OnRemoteDetonatorExpired`) 10.0)
              (`self.K2_DestroyActor` _asbp_power_up_remote_detonator))))))))

(event `OnRemoteDetonatorExpired`
  (`self.SetRemoteDetonatorActive` false))

(fn `UserConstructionScript`)