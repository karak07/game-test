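; Game mode for a local two-player Bomberman game that sets up both players and runs a timed round.
; SetupPlayers creates a second local player if needed, restarts both at separate PlayerStarts and tints their body materials red and green.
; A looping one-second timer updates the countdown string and ends the round when time runs out or either pawn's collision is disabled, a temporary death check.
; FinishRound pauses the game and fires a round-finished event.
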(event `self.ReceiveBeginPlay`
  (`parent.ReceiveBeginPlay`)
  (`self.SetupPlayers`)
  ;[1 1 1] Setting up Round Timer
  (bind _returnvalue (`KismetSystemLibrary.K2_SetTimerDelegate` (delegate `OnRoundTimerTick`) 1.0 true))
  (set `self.RoundTimerHandle` _returnvalue)
  (`self.UpdateRoundTimer`))

(event `OnRoundTimerTick`
  ;[1 1 1] Setting up Round Timer
  (`self.UpdateRoundTimer`)
  (if (== (`self.RoundTimer`) 0)
    (`self.FinishRound` :!label _label)
    (elif (or (not (`self.GetActorEnableCollision` (`GameplayStatics.GetPlayerPawn` 0))) (not (`self.GetActorEnableCollision` (`GameplayStatics.GetPlayerPawn` 1))))
      (goto _label))))

(fn `FinishRound`
  (`GameplayStatics.SetGamePaused` true)
  (set `self.RoundFinished` true)
  (`self.RoundFinishedEvent`))

(fn `SetupPlayers`
  (locals (PlayerStarts :type "Array of PlayerStart Object Reference"))
  ;[1 1 1] Selecting 1st spawn location
  (bind _outactors (`GameplayStatics.GetAllActorsOfClass` "/Script/Engine.PlayerStart"))
  (bind _output_get (set `local.PlayerStarts` _outactors))
  (`self.RestartPlayerAtPlayerStart` (`GameplayStatics.GetPlayerController` 0) (`|GetArrayItem` _output_get))
  ;[1 1 1] Changing Color of 1st Pawn
  (bind _ascharacter (cast `Character` (`Controller.K2_GetPawn` (`GameplayStatics.GetPlayerController` 0))))
  (`MeshComponent.SetVectorParameterValueOnMaterials` (`Character.Mesh` _ascharacter) "BodyColor" (`KismetMathLibrary.Conv_LinearColorToVector` (make `LinearColor` 1.0)))
  ;[1 1 1] Creating 2nd Player
  (bind _returnvalue (`self.GetNumPlayers`))
  (if (< _returnvalue 2)
    (`GameplayStatics.CreatePlayer` -1))
  ;[1 1 1] Selecting 2nd spawn location
  (`self.RestartPlayerAtPlayerStart` (`GameplayStatics.GetPlayerController` 1) (`|GetArrayItem` (`local.PlayerStarts`) 1))
  ;[1 1 1] Changing Color of 2nd Pawn
  (bind _ascharacter_2 (cast `Character` (`Controller.K2_GetPawn` (`GameplayStatics.GetPlayerController` 1))))
  (`MeshComponent.SetVectorParameterValueOnMaterials` (`Character.Mesh` _ascharacter_2) "BodyColor" (`KismetMathLibrary.Conv_LinearColorToVector` (make `LinearColor` 0.0 1.0))))

(fn `UpdateRoundTimer`
  (bind _roundtimer (`self.RoundTimer`))
  (if (> _roundtimer 0)
    (bind _result (`/Engine/EditorBlueprintResources/StandardMacros.DecrementInt` _roundtimer)
      (:`  `
        (bind _returnvalue (`BombermanBFL.FormatAsTime` _result))
        (set `self.RoundTimerString` _returnvalue)))))

(fn `UserConstructionScript`)